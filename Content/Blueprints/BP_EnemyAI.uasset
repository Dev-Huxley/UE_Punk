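; Enemy AI Blueprint that chases the player on sight and plays an attack montage when within range.
; Pawn sensing latches IsSeeingPlayer and calls FollowPlayer, which issues AIMoveTo toward the player character and checks attack range immediately, without waiting for arrival.
; CanAttack and a montage-playing check gate the attack, with a delay matching the montage length.
; Tick halts movement until a pawn is first seen.
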(event `self.ReceiveTick`
  (params (DeltaSeconds :type "Float (single-precision)"))
  (if (not (`self.isSeeingPlayer?`))
    (`MovementComponent.StopMovementImmediately` (`self.CharacterMovement`))))

(event `self.PawnSensing.OnSeePawn`
  (params (Pawn :type "Pawn Object Reference"))
  ; 폰 발견 이벤트
  (set `self.isSeeingPlayer?` true)
  (`self.FollowPlayer`))

(event `FollowPlayer`
  (set `self.canAttack?` true)
  (if (`self.isSeeingPlayer?`)
    (`|AIMoveTo` self (0.0 0.0 0.0) (`GameplayStatics.GetPlayerCharacter` 0)
      (:`then`
        (if (`self.canAttack?`)
          (set `self.canAttack?` false)
          (if (< (`self.GetDistanceTo` (`GameplayStatics.GetPlayerPawn` 0)) (`self.attackRange`))
            (if (not (`AnimInstance.Montage_IsPlaying` (`SkeletalMeshComponent.GetAnimInstance` (`self.Mesh`)) "/Game/Animations/AI/Montage.Montage"))
              (bind _returnvalue (`self.PlayAnimMontage` "/Game/Animations/AI/Montage.Montage"))
              (`KismetSystemLibrary.Delay` _returnvalue)
              (set `self.canAttack?` true))
            (else
              (set `self.canAttack?` true))))))
    (else
      (set `self.isSeeingPlayer?` false))))

(fn `UserConstructionScript`)