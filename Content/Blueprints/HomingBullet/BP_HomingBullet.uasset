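; BP_HomingBullet is a projectile that turns homing after a short random delay and damages BP_Enemy actors.
; BeginPlay enables homing on ProjectileMovement after the delay and caches the player pawn, but sets no homing target.
; Sphere overlap filters by a cast to BP_Enemy, applies small random damage with the player pawn as causer, spawns an explosion, prints a debug string and destroys the bullet.
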(event `self.ReceiveBeginPlay`
  (bind _projectilemovement (`self.ProjectileMovement`))
  ; ~초 지난 뒤 유도로 전환
  (`KismetSystemLibrary.Delay` (`KismetMathLibrary.RandomFloatInRange` 0.2 0.5))
  (set `ProjectileMovementComponent.bIsHomingProjectile` true _projectilemovement)
  (set `ProjectileMovementComponent.HomingAccelerationMagnitude` 9000.0 _projectilemovement)
  (set `self.PlayerCharacter` (`GameplayStatics.GetPlayerPawn` 0)))

(event `self.Sphere.OnComponentBeginOverlap`
  (params (OverlappedComponent :type "PrimitiveComponent Object Reference") (OtherActor :type "Actor Object Reference") (OtherComp :type "PrimitiveComponent Object Reference") (OtherBodyIndex :type Integer) (bFromSweep :type Boolean) (SweepResult :type "HitResult Structure (by ref)"))
  ; Enemy태그 체크하고 맞다면 destroy+emitter
  (bind _asbp_enemy (cast `/Game/CustomContents/Blueprints/Character/Enemy/BP_Enemy` OtherActor))
  (bind _output_get (set `self.Damage` (`KismetMathLibrary.RandomFloatInRange` 1.0 3.0)))
  (`GameplayStatics.ApplyDamage` _asbp_enemy _output_get null (`self.PlayerCharacter`))
  (`GameplayStatics.SpawnEmitterAtLocation` "/Game/StarterContent/Particles/P_Explosion.P_Explosion" (`self.K2_GetActorLocation`))
  (`KismetSystemLibrary.PrintString` "Hello")
  (`self.K2_DestroyActor`))

(fn `UserConstructionScript`)