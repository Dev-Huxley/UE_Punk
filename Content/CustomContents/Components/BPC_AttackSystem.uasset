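; Player attack component handling pistol fire, reload and melee hit traces, pulling stats and ammo from the player's stat system.
; IA_Attack checks fire delay and reload lock, then fires a projectile toward a spread-randomized line trace, injects look input as recoil and updates UI, or reloads when empty.
; Timer-triggered sphere traces from alternating hands damage BP_Enemy.
; The weapon-type branch and four-hit montage combo are disconnected, so never run.
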(event `self.ReceiveBeginPlay`
  (`|ExecutionSequence`
    (:`then_0`
      ; Init Player
      (bind _asbp_player_character (cast `/Game/CustomContents/Blueprints/Character/Player/BP_PlayerCharacter` (`self.GetOwner`)))
      (bind _output_get (set `self.PlayerCharacter` _asbp_player_character))
      (set `self.CharacterMesh` (`Character.Mesh` _output_get)))
    (:`then_1`
      ; Init Bullet Spawn Location
      (set `self.Bullet Spawn Location` (`/Game/CustomContents/Blueprints/Character/Player/BP_PlayerCharacter.BulletSpawnLocation` (`self.PlayerCharacter`))))
    (:`then_2`
      ; InitStat
      (bind _output_get_2 (set `self.BPC Player Stat System` (`/Game/CustomContents/Blueprints/Character/Player/BP_PlayerCharacter.BPC_PlayerStatSystem` (`self.PlayerCharacter`))))
      (`/Game/CustomContents/Components/BPC_PlayerStatSystem.InitData` _output_get_2)
      (set `self.Attack Radius` (`/Game/CustomContents/Components/BPC_PlayerStatSystem.AttackRadius` _output_get_2))
      (set `self.FireRate` (`/Game/CustomContents/Components/BPC_PlayerStatSystem.FireRate` _output_get_2)))
    (:`then_3`
      ; SET BP_UI
      (bind _returnvalue (`GameplayStatics.GetActorOfClass` "/Game/CustomContents/UI/BP/BP_UI.BP_UI_C"))
      (set `self.BP_UI` _returnvalue))))

(event `ResetByHit`
  ; ResetByHit
  (if (`/Game/CustomContents/Blueprints/Character/Player/BP_PlayerCharacter.IsHitting` (`self.PlayerCharacter`))
    (set `self.IsAttacking` false)
    (set `self.ComboCounter` 0)))

(event `EnhancedInput|/Game/CustomContents/Input/IA_Reload`
  (params (ActionValue :type Boolean) (ElapsedSeconds :type "Float (double-precision)") (TriggeredSeconds :type "Float (double-precision)") (InputAction :type "InputAction Object Reference" :default "/Game/CustomContents/Input/IA_Reload.IA_Reload"))
  (bind _bpc_userinterface (`/Game/CustomContents/Blueprints/Character/Player/BP_PlayerCharacter.BPC_UserInterface` (`self.PlayerCharacter`)))
  ; 총 들고 있을때 리로드 검증
  (:`Triggered`
    (if (`|EnumEquality` (`/Game/CustomContents/Blueprints/Character/Player/BP_PlayerCharacter.CurrentWeaponType` (`self.PlayerCharacter`)) "NewEnumerator3")
      ; OnInputAction_GunFire
      (`|PlayMontage` (`self.CharacterMesh`) "/Game/Characters/Mannequins/Anims/Pistol/MM_Pistol_Reload_Montage.MM_Pistol_Reload_Montage" :!label _label
        (:`then`
          ; Reload Lock
          (set `self.Reloading` true)
          (`KismetSystemLibrary.Delay` 3.0)
          (set `self.Reloading` false))
        (:`OnCompleted`
          (bind (_equipbullet _hasbullet) (`/Game/CustomContents/Components/BPC_PlayerStatSystem.ReloadBullets` (`/Game/CustomContents/Blueprints/Character/Player/BP_PlayerCharacter.BPC_PlayerStatSystem` (`self.PlayerCharacter`)) :!label _label_2))
          (set `self.CanFire` true)
          (`/Game/CustomContents/UI/BP/BPC_UserInterface.OnUpdateEquipBullet` _bpc_userinterface _equipbullet)
          (`/Game/CustomContents/UI/BP/BPC_UserInterface.OnUpdateHasBullet` _bpc_userinterface _hasbullet)
          ; EFX_Reload
          (if (`|EnumInequality` (`/Game/CustomContents/UI/BP/BP_UI.CombatState` (`self.BP_UI`)) "NewEnumerator2")
            (`GameplayStatics.PlaySound2D` "/Game/CustomContents/UI/Sound/WAV_ReloadGun01.WAV_ReloadGun01" 1.0 1.0 0.0 null null)))
        (:`OnInterrupted`
          (goto _label_2))))))

(event `ResetCounter`
  ; ComboAttackSequence
  (set `self.ComboCounter` 0))

(event `self.ReceiveTick`
  (params (DeltaSeconds :type "Float (single-precision)"))
  ; Tick
  (set `self.ElapsedTime` (+ DeltaSeconds (`self.ElapsedTime`))))

(event `EnhancedInput|/Game/CustomContents/Input/IA_Attack`
  (params (ActionValue :type Boolean) (ElapsedSeconds :type "Float (double-precision)") (TriggeredSeconds :type "Float (double-precision)") (InputAction :type "InputAction Object Reference" :default "/Game/CustomContents/Input/IA_Attack.IA_Attack"))
  (bind _playercharacter (`self.PlayerCharacter`))
  (bind _bullet_spawn_location (`self.Bullet Spawn Location`))
  (bind _returnvalue (`SceneComponent.K2_GetComponentLocation` _bullet_spawn_location))
  (bind (_returnvalue_x _returnvalue_y) (`KismetMathLibrary.BreakVector2D` (`KismetMathLibrary.MakeVector2D` (`KismetMathLibrary.RandomFloatInRange` -0.5 0.5) (`KismetMathLibrary.RandomFloatInRange` -0.2 -0.5))))
  (bind _returnvalue_2 (`SceneComponent.K2_GetComponentLocation` (`/Game/CustomContents/Blueprints/Character/Player/BP_PlayerCharacter.FireSpawnLocation` (`self.PlayerCharacter`))))
  ; OnAttack
  (:`Triggered`
    ; FireEnable?
    (if (`self.IsFireEnable`)
      (set `self.ElapsedTime` 0.0)
      (set `self.CanFire` false)
      ; OnInputAction_GunFire
      (`|PlayMontage` (`self.CharacterMesh`) "/Game/Characters/Mannequins/Anims/Pistol/MM_Pistol_Fire_Montage1.MM_Pistol_Fire_Montage1" (`self.FireRate`)
        (:`then`
          (bind _fire_ (`/Game/CustomContents/Components/BPC_PlayerStatSystem.RedundancyBullet` (`/Game/CustomContents/Blueprints/Character/Player/BP_PlayerCharacter.BPC_PlayerStatSystem` (`self.PlayerCharacter`)))) ; 장전되어있는 탄 확인
          (if _fire_
            (bind _outhit (`KismetSystemLibrary.LineTraceSingle` _returnvalue (+ _returnvalue (* (`KismetMathLibrary.RandomUnitVectorInConeInDegrees` (`SceneComponent.GetForwardVector` _bullet_spawn_location) (`self.SpreadAngle`)) (`self.MaxRange`))) "TraceTypeQuery1")) ; Bullet Spawn Location에서 라인트레이싱
            (bind _returnvalue_3 (`KismetMathLibrary.FindLookAtRotation` _returnvalue (`.Location` (`GameplayStatics.BreakHitResult` _outhit))))
            (`|SpawnActorFromClass` "/Game/POLYMORPHFX/DemolitionistGunnerFireShotVFX/Blueprints/BP_Demolitionist_Gunner_FireShot_Projectile_01.BP_Demolitionist_Gunner_FireShot_Projectile_01_C" (`KismetMathLibrary.MakeTransform` _returnvalue_2 _returnvalue_3 (0.5 0.5 0.5)) "Undefined" "MultiplyWithRoot" null null)
            (`EnhancedInputSubsystemInterface.InjectInputForAction` :`self` (pcsubsystem `EnhancedInputLocalPlayerSubsystem` (`GameplayStatics.GetPlayerController` 0)) :`Action` "/Game/CustomContents/Input/IA_LookAround.IA_LookAround" :`RawValue` (`EnhancedInputLibrary.MakeInputActionValueOfType` _returnvalue_x _returnvalue_y 0.0 "Axis2D"))
            (`NiagaraFunctionLibrary.SpawnSystemAtLocation` "/Game/POLYMORPHFX/DemolitionistGunnerFireShotVFX/Niagara/NS_Demolitionist_Gunner_FireShot_Muzzleflash_01.NS_Demolitionist_Gunner_FireShot_Muzzleflash_01" _returnvalue_2 _returnvalue_3 (0.1 0.1 0.1))
            (bind _equip_bullet (`/Game/CustomContents/Components/BPC_PlayerStatSystem.DecreaseBullet` (`/Game/CustomContents/Blueprints/Character/Player/BP_PlayerCharacter.BPC_PlayerStatSystem` _playercharacter)))
            ; ComboAttackSequence
            (`/Game/CustomContents/UI/BP/BPC_UserInterface.OnUpdateEquipBullet` (`/Game/CustomContents/Blueprints/Character/Player/BP_PlayerCharacter.BPC_UserInterface` _playercharacter) _equip_bullet)
            ; OnShot
            (`/Game/CustomContents/UI/BP/BPC_UserInterface.OnShot` (`/Game/CustomContents/Blueprints/Character/Player/BP_PlayerCharacter.BPC_UserInterface` (`self.PlayerCharacter`)))
            ; EFX_Shot
            (if (`|EnumInequality` (`/Game/CustomContents/UI/BP/BP_UI.CombatState` (`self.BP_UI`)) "NewEnumerator2")
              (`GameplayStatics.PlaySound2D` "/Game/CustomContents/UI/Sound/WAV_PistolShot01.WAV_PistolShot01" 1.0 1.0 0.0 null null))
            (else
              (goto _label))))
        (:`OnCompleted`
          (set `self.CanFire` true))))))

(event `StopAttackTrace`
  ; OnStopAttackTrace
  (`KismetSystemLibrary.K2_ClearAndInvalidateTimerHandle` (`self.AttackTimerHandler`)) ; 이벤트가 실행되면 실행되어 있는 타이머는 해제
)

(event `StartAttackTrace`
  ; OnStartAttackTrace
  (bind _returnvalue (`KismetSystemLibrary.K2_SetTimerDelegate` (delegate `AttackTrace`) 0.01))
  (set `self.AttackTimerHandler` _returnvalue))

(event `AttackTrace`
  (bind (_start _end) (`self.Get Hand Location` (`/Game/CustomContents/Blueprints/Character/Player/BP_PlayerCharacter.RightHand` (`self.PlayerCharacter`))))
  (bind (_start_2 _end_2) (`self.Get Hand Location` (`/Game/CustomContents/Blueprints/Character/Player/BP_PlayerCharacter.LeftHand` (`self.PlayerCharacter`))))
  ; OnStartAttackTrace
  (switch `int` (`self.ComboCounter`) ; 0, 2 : Left\n1, 3 : Right
    (:`0`
      ;;[0 0.03788 0.15 0.5] Attack_LeftHand
      (bind (_damage _critical) (`/Game/CustomContents/Components/BPC_PlayerStatSystem.GetDamage` (`/Game/CustomContents/Blueprints/Character/Player/BP_PlayerCharacter.BPC_PlayerStatSystem` (`self.PlayerCharacter`)) :!label _label_3))
      (`self.Attack Sphere Trace` _start_2 _end_2 _damage _critical (`self.Attack Radius`)))
    (:`1`
      (bind (_damage_2 _critical_2) (`/Game/CustomContents/Components/BPC_PlayerStatSystem.GetDamage` (`/Game/CustomContents/Blueprints/Character/Player/BP_PlayerCharacter.BPC_PlayerStatSystem` (`self.PlayerCharacter`)) :!label _label_4))
      ;;[0.15 0 0.02109 0.5] Attack_RightHand
      (`self.Attack Sphere Trace` _start _end _damage_2 _critical_2 (`self.Attack Radius`)))
    (:`2`
      (goto _label_3))
    (:`3`
      (goto _label_4))))

(fn `Attack Sphere Trace`
  (params (Start :type "Vector Structure") (End :type "Vector Structure") (Damage :type "Float (single-precision)") (Critical :type Boolean) (AttackRadius :type "Float (double-precision)") (DrawDebug :type "EDrawDebugTrace Enum" :default "None"))
  (bind (_outhit _returnvalue) (`KismetSystemLibrary.SphereTraceSingle` :`Start` Start :`End` End :`Radius` AttackRadius :`TraceChannel` "TraceTypeQuery1" :`DrawDebugType` DrawDebug :`TraceColor` (struct :`G` 0.036216 :`B` 1.0 :`A` 1.0) :`TraceHitColor` (struct :`R` 0.284729 :`G` 0.322319 :`B` 1.0 :`A` 1.0) :`DrawTime` 7.0))
  (if _returnvalue
    (bind _asbp_enemy (cast `/Game/CustomContents/Blueprints/Character/Enemy/BP_Enemy` (`.HitActor` (`GameplayStatics.BreakHitResult` _outhit)))
      (:`then`
        (`/Game/CustomContents/Blueprints/Character/Enemy/BP_Enemy.OnDamage` _asbp_enemy Damage Critical (`Pawn.GetController` (`self.PlayerCharacter`)) (`self.PlayerCharacter`)))
      (:`CastFailed`
        (`KismetSystemLibrary.PrintString` "Enemy Cast Failed" false false)))
    (else
      (`KismetSystemLibrary.PrintString` "Player Attack Failed" false false))))

(fn `DetectLookAtTarget`
  (params (DetectRange :type "Float (double-precision)") (DetectRadius :type "Float (double-precision)"))
  (returns (Detect :type Boolean) (Enemy :type "/Game/CustomContents/Blueprints/Character/Enemy/BP_Enemy Object Reference"))
  (locals (Radius :type "Float (double-precision)") (Range :type "Float (double-precision)"))
  (bind _returnvalue (`GameplayStatics.GetPlayerCameraManager` 0))
  (bind _returnvalue_2 (`PlayerCameraManager.GetCameraLocation` _returnvalue))
  (set `local.Range` DetectRange)
  (set `local.Radius` DetectRadius)
  (bind (_outhit _returnvalue_3) (`KismetSystemLibrary.SphereTraceSingle` _returnvalue_2 (+ _returnvalue_2 (* (`KismetMathLibrary.GetForwardVector` (`PlayerCameraManager.GetCameraRotation` _returnvalue)) (`local.Range`))) (`local.Radius`) "TraceTypeQuery1"))
  (if _returnvalue_3
    (bind (_bblockinghit _binitialoverlap _time _distance _location _impactpoint _normal _impactnormal _physmat _hitactor) (`GameplayStatics.BreakHitResult` _outhit))
    (if (`Actor.ActorHasTag` _hitactor "Enemy")
      (bind _asbp_enemy (cast `/Game/CustomContents/Blueprints/Character/Enemy/BP_Enemy` _hitactor)
        (:`then`
          (return true _asbp_enemy))
        (:`CastFailed`
          (return false null)))
      (else
        (return false null)))
    (else
      (return false null))))

(fn `Get Hand Location`
  (params (Hand :type "SceneComponent Object Reference"))
  (returns (Start :type "Vector Structure") (End :type "Vector Structure"))
  (return (`SceneComponent.K2_GetComponentLocation` Hand) (`KismetMathLibrary.TransformLocation` (`SceneComponent.K2_GetComponentToWorld` Hand) (+ (`SceneComponent.RelativeLocation` Hand) (20.0 0.0 0.0)))))

(fn `IsFireEnable`
  (returns (Enable :type Boolean))
  (if (and (>= (`self.ElapsedTime`) (`self.FireDelay`)) (== (`self.Reloading`) false))
    (return true)
    (else
      (return false))))

(fn `ResetCanFire`
  (set `self.CanFire` true))