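; Stat component for enemies that tracks health, strength and critical stats, and identifies boss or slave type.
; BeginPlay loads boss stats from PunkGameInstance, while InitSlave switches the type to slave and loads slave stats.
; GetDamage rolls 85–115% of Strength, multiplied on a random critical.
; Health functions clamp the value and report death or percentage; IncreaseHealth updates the passed HUD only upon reaching maximum, DecreaseHealth every time.
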(event `self.ReceiveBeginPlay`
  (bind _aspunk_game_instance (cast `/Game/CustomContents/Blueprints/PunkGameInstance` (`GameplayStatics.GetGameInstance`)))
  ; SetData
  (`|ExecutionSequence`
    (:`then_0`
      (bind (_statdata_hp _statdata_atk _statdata_cri_rate _statdata_cri_value) (break `/Game/CustomContents/MasterData/BossStatData` (`/Game/CustomContents/Blueprints/PunkGameInstance.GetBossStat` _aspunk_game_instance)))
      (set `self.MaxHealth` (`KismetMathLibrary.Conv_IntToDouble` _statdata_hp)))
    (:`then_1`
      (set `self.Strength` (`KismetMathLibrary.Conv_IntToDouble` _statdata_atk)))
    (:`then_2`
      (set `self.CriticalRate` _statdata_cri_rate))
    (:`then_3`
      (set `self.CriticalValue` _statdata_cri_value))
    (:`then_4`
      (`self.InitializeStat`))))

(fn `DecreaseHealth`
  (params (`Damage Point` :type "Float (double-precision)") (`Player HUD` :type "/Game/CustomContents/UI/WB/Combat/WB_HUD Object Reference"))
  (returns (IsDead :type Boolean))
  (bind _returnvalue (- (`self.CurrentHealth`) `Damage Point`))
  (if (< _returnvalue 0.0)
    (set `self.CurrentHealth` 0.0)
    (else
      (set `self.CurrentHealth` _returnvalue)))
  (`self.DisplayHealth` `Player HUD`)
  (if (<= (`self.CurrentHealth`) 0.0)
    (bind _output_get (set `self.IsDead` true))
    (return _output_get)
    (else
      (bind _output_get_2 (set `self.IsDead` false))
      (return _output_get_2))))

(fn `DisplayHealth`
  (params (HUD :type "/Game/CustomContents/UI/WB/Combat/WB_HUD Object Reference"))
  (`/Engine/EditorBlueprintResources/StandardMacros.IsValid` HUD
    (:`Is Valid`
      (`/Game/CustomContents/UI/WB/Combat/WB_HUD.SetHealthBarPercent` HUD (`self.CurrentHealth`) (`self.MaxHealth`)))))

(fn `GetDamage`
  (returns (Damage :type "Float (double-precision)") (Critical :type Boolean))
  (locals (ActivateCritical :type Boolean))
  (bind _strength (`self.Strength`))
  (bind _strength_2 (`self.Strength`))
  ;[0.15 0.01305 0 0.5] Calc CriticalRate
  (bind _output_get (set `local.ActivateCritical` (<= (`KismetMathLibrary.RandomFloatInRange` 0.0 100.0) (`self.CriticalRate`))))
  (if _output_get
    (return (`KismetMathLibrary.Conv_IntToDouble` (`KismetMathLibrary.FTrunc` (* (`KismetMathLibrary.RandomFloatInRange` (* _strength_2 0.85) (* _strength_2 1.15)) (`self.CriticalValue`)))) (`local.ActivateCritical`))
    (else
      (return (`KismetMathLibrary.Conv_IntToDouble` (`KismetMathLibrary.FTrunc` (`KismetMathLibrary.RandomFloatInRange` (* _strength 0.85) (* _strength 1.15)))) (`local.ActivateCritical`)))))

(fn `HealthPercent`
  (returns (HealthPercent :type "Float (double-precision)"))
  (return (/ (`self.CurrentHealth`) (`self.MaxHealth`))))

(fn `IncreaseHealth`
  (params (HealthPoint :type "Float (double-precision)") (`Player HUD` :type "/Game/CustomContents/UI/WB/Combat/WB_HUD Object Reference"))
  (set `self.CurrentHealth` (+ HealthPoint (`self.CurrentHealth`)))
  (if (>= (`self.CurrentHealth`) (`self.MaxHealth`))
    (set `self.CurrentHealth` (`self.MaxHealth`))
    (`self.DisplayHealth` `Player HUD`)))

(fn `InitializeStat`
  (set `self.CurrentHealth` (`self.MaxHealth`))
  (`self.DisplayHealth` null))

(fn `InitSlave`
  (set `self.EnemyType` "NewEnumerator0")
  (bind _aspunk_game_instance (cast `/Game/CustomContents/Blueprints/PunkGameInstance` (`GameplayStatics.GetGameInstance`)))
  ; SetData
  (`|ExecutionSequence`
    (:`then_0`
      (bind (_statdata_hp _statdata_atk _statdata_cri_rate _statdata_cri_value) (break `/Game/CustomContents/MasterData/SlaveStatData` (`/Game/CustomContents/Blueprints/PunkGameInstance.GetSlaveStat` _aspunk_game_instance)))
      (set `self.MaxHealth` (`KismetMathLibrary.Conv_IntToDouble` _statdata_hp)))
    (:`then_1`
      (set `self.Strength` (`KismetMathLibrary.Conv_IntToDouble` _statdata_atk)))
    (:`then_2`
      (set `self.CriticalRate` _statdata_cri_rate))
    (:`then_3`
      (set `self.CriticalValue` _statdata_cri_value))
    (:`then_4`
      (`self.InitializeStat`))))

(fn `IsBossType`
  (returns (IsBoss :type Boolean))
  (locals (NewLocalVar :type Byte))
  (return (`|EnumEquality` (`self.EnemyType`) "NewEnumerator1")))