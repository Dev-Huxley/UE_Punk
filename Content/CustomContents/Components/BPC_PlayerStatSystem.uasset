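; Player stat component that manages health and death, attack damage and gun ammo.
; Health starts at max on BeginPlay and is clamped on change, with damage returning a death flag.
; Melee and bullet damage roll 85–115% of Strength or GunStrength, with a random critical multiplier.
; Reloading moves reserve rounds into the gun, and debug prints stand in for health/ammo display and reload feedback.
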(event `self.ReceiveBeginPlay`
  (`self.InitializeStat`))

(fn `DecreaseBullet`
  ;[0.4323 0.4323 0.4323 0] 사격 후 장탄수 감소
  (bind _result (`/Engine/EditorBlueprintResources/StandardMacros.DecrementInt` (`self.EquipBullet`))
    (:`  `
      (`KismetSystemLibrary.PrintString` (`KismetTextLibrary.Conv_TextToString` (`|FormatText` "장탄 수 : {Equip Bullet}" _result))))))

(fn `DecreaseHealth`
  (params (`Damage Point` :type "Float (double-precision)"))
  (returns (IsDead :type Boolean))
  (bind _returnvalue (- (`self.CurrentHealth`) `Damage Point`))
  (if (< _returnvalue 0.0)
    (set `self.CurrentHealth` 0.0)
    (else
      (set `self.CurrentHealth` _returnvalue)))
  (`self.DisplayHealth`)
  (if (<= (`self.CurrentHealth`) 0.0)
    (set `self.CurrentHealth` 0.0)
    (bind _output_get (set `self.IsDead` true))
    (return _output_get)
    (else
      (bind _output_get_2 (set `self.IsDead` false))
      (return _output_get_2))))

(fn `DisplayHealth`
  (`KismetSystemLibrary.PrintString` (`KismetStringLibrary.Concat_StrStr` (`KismetStringLibrary.Concat_StrStr` (`KismetStringLibrary.Conv_DoubleToString` (`self.CurrentHealth`)) "/") (`KismetStringLibrary.Conv_DoubleToString` (`self.MaxHealth`)))))

(fn `GetBulletDamage`
  (returns (Damage :type "Float (double-precision)") (Critical :type Boolean))
  (locals (ActivateCritical :type Boolean))
  (bind _gunstrength (`self.GunStrength`))
  (bind _gunstrength_2 (`self.GunStrength`))
  ;[0.15 0.01305 0 0.5] Calc CriticalRate
  (bind _output_get (set `local.ActivateCritical` (<= (`KismetMathLibrary.RandomFloatInRange` 0.0 100.0) (`self.CriticalRate`))))
  (if _output_get
    (return (`KismetMathLibrary.Conv_IntToDouble` (`KismetMathLibrary.FTrunc` (* (`KismetMathLibrary.RandomFloatInRange` (* _gunstrength 0.85) (* _gunstrength 1.15)) (`self.CriticalValue`)))) (`local.ActivateCritical`))
    (else
      (return (`KismetMathLibrary.Conv_IntToDouble` (`KismetMathLibrary.FTrunc` (`KismetMathLibrary.RandomFloatInRange` (* _gunstrength_2 0.85) (* _gunstrength_2 1.15)))) (`local.ActivateCritical`)))))

(fn `GetDamage`
  (returns (Damage :type "Float (double-precision)") (Critical :type Boolean))
  (locals (ActivateCritical :type Boolean))
  (bind _strength (`self.Strength`))
  (bind _strength_2 (`self.Strength`))
  ;[0.15 0.01305 0 0.5] Calc CriticalRate
  (bind _output_get (set `local.ActivateCritical` (<= (`KismetMathLibrary.RandomFloatInRange` 0.0 100.0) (`self.CriticalRate`))))
  (if _output_get
    (return (`KismetMathLibrary.Conv_IntToDouble` (`KismetMathLibrary.FTrunc` (* (`KismetMathLibrary.RandomFloatInRange` (* _strength_2 0.85) (* _strength_2 1.15)) (`self.CriticalValue`)))) (`local.ActivateCritical`))
    (else
      (return (`KismetMathLibrary.Conv_IntToDouble` (`KismetMathLibrary.FTrunc` (`KismetMathLibrary.RandomFloatInRange` (* _strength 0.85) (* _strength 1.15)))) (`local.ActivateCritical`)))))

(fn `IncreaseHealth`
  (params (HealthPoint :type "Float (double-precision)"))
  (set `self.CurrentHealth` (+ HealthPoint (`self.CurrentHealth`)))
  (if (>= (`self.CurrentHealth`) (`self.MaxHealth`))
    (set `self.CurrentHealth` (`self.MaxHealth`))
    (`self.DisplayHealth`)))

(fn `InitializeStat`
  (set `self.CurrentHealth` (`self.MaxHealth`))
  (`self.DisplayHealth`))

(fn `RedundancyBullet`
  (returns (`Fire?` :type Boolean))
  (return (> (`self.EquipBullet`) 0)))

(fn `RelaodBullet`
  (bind _equipbullet (`self.EquipBullet`))
  (bind _returnvalue (- (`self.ReloadBullet`) _equipbullet))
  (bind _returnvalue_2 (> (`self.EquipBullet`) 0))
  (if (not (== (`self.EquipBullet`) 6))
    ; R키 눌러서 장전했는지 검증
    (if _returnvalue_2
      (bind _output_get (set `self.bReload` _returnvalue_2)))
    ; 총 잔여탄 갯수 검증
    (if (>= (`self.HasBullet`) (`self.ReloadBullet`))
      ; R키 누르고 장탄 수 1~5 검증
      (if _output_get
        (`KismetSystemLibrary.PrintString` "장전모션")
        ; 장탄 수에 맞게 장전하고 장전 수 만큼 잔여탄 정리
        (bind _output_get_2 (set `self.TempBullet` _returnvalue))
        (set `self.EquipBullet` (+ _returnvalue _equipbullet))
        (bind _output_get_3 (set `self.HasBullet` (- (`self.HasBullet`) _output_get_2)))
        (`KismetSystemLibrary.PrintText` (`|FormatText` "장전완료, 남은 탄: {Has Bullet}" _output_get_3))
        (else
          (`KismetSystemLibrary.PrintString` "장전모션 ")
          ; 장탄 수 0발이고 잔여 탄이 전부 있을때 자동으로 장전
          (set `self.EquipBullet` (`self.ReloadBullet`))
          (bind _output_get_4 (set `self.HasBullet` (- (`self.HasBullet`) (`self.ReloadBullet`))))
          (`KismetSystemLibrary.PrintText` (`|FormatText` "장전완료, 남은 탄: {Has Bullet}" _output_get_4))))
      (else
        ; 총 잔여탄 1~5 검증
        (if (> (`self.HasBullet`) 0)
          (`KismetSystemLibrary.PrintString` "장전모션")
          ; 남은 탄만큼 장전
          (set `self.EquipBullet` (+ (`self.HasBullet`) (`self.EquipBullet`)))
          (set `self.HasBullet` 0)
          (`KismetSystemLibrary.PrintString` "장전완료, 탄 소진")
          (else
            ; 장전불가
            (`KismetSystemLibrary.PrintString` "틱틱 거리는 소리나 모션")))))
    ; 장전 키 리셋
    (set `self.bReload` false)))