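; Enemy combat component for BP_Enemy that drives chasing and melee attacks through a simple state machine.
; Tick measures target distance, turns and moves the enemy while chasing, and switches to Attack within range unless hit or dead.
; Each chase locks direction and duration on entry, then moves by setting actor location without sweep.
; Attack snaps toward the target and plays a dual-weapon combo montage, returning to Chase when it completes or is interrupted.
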(event `self.ReceiveBeginPlay`
  ;[0.1337 0.15 0 0.5] BeginPlay
  (bind _asbp_enemy (cast `/Game/CustomContents/Blueprints/Character/Enemy/BP_Enemy` (`self.GetOwner`)))
  (set `self.EnemyCharacter` _asbp_enemy))

(event `StartDash`
  ; StartDash
  (if (not (`self.IsDashing`))
    (set `self.IsDashing` true)
    (bind _targetcharacter (`/Game/CustomContents/Blueprints/Character/Enemy/BP_Enemy.TargetCharacter` (`self.EnemyCharacter`))
      (:`then`
        (set `self.DashDirection` (`KismetMathLibrary.Normal` (- (`Actor.K2_GetActorLocation` _targetcharacter) (`Actor.K2_GetActorLocation` (`self.EnemyCharacter`)))))
        (`KismetSystemLibrary.PrintString` "Start Dash Called"))
      (:`else`))))

(event `self.ReceiveTick`
  (params (DeltaSeconds :type "Float (single-precision)"))
  ;[0.15 0.05441 0.0927 0.5] Tick
  (`self.CalcDistanceToTarget`)
  (`KismetSystemLibrary.PrintString` (`|GetEnumeratorNameAsString` (`self.CurrentState`)) true true (struct :`R` 0.890681 :`G` 0.001397 :`B` 1.0 :`A` 1.0) 2.0 "1")
  (`|ExecutionSequence`
    (:`then_0`
      (switch `/Game/CustomContents/Components/EEnemyState` (`self.CurrentState`)
        (:`NewEnumerator5`
          (`self.RotateToTarget`)
          (`self.MovingTowardPlayer`))))
    (:`then_1`
      ;; 타겟과의 거리가 MinChaseDistance보다 작고 IsHit==false이고 IsDead==false이면 근접공격
      (if (and (< (`self.DistanceToTarget`) (`self.MinChaseDistance`)) (not (`/Game/CustomContents/Blueprints/Character/Enemy/BP_Enemy.IsHit` (`self.EnemyCharacter`))) (not (`/Game/CustomContents/Blueprints/Character/Enemy/BP_Enemy.Is Dead` (`self.EnemyCharacter`))))
        (`/Game/CustomContents/Blueprints/Character/Enemy/BP_Enemy.TargetCharacter` (`self.EnemyCharacter`)
          (:`then`
            (`self.SetCurrentState` "NewEnumerator3"))
          (:`else`))))))

(event `DualComboAttack`
  (bind _enemycharacter (`self.EnemyCharacter`))
  ; DualComboAttack
  (if (`|EnumInequality` (`self.CurrentState`) "NewEnumerator6")
    (bind _targetcharacter (`/Game/CustomContents/Blueprints/Character/Enemy/BP_Enemy.TargetCharacter` _enemycharacter)
      (:`then`
        (`KismetSystemLibrary.PrintString` "Dual Combo Attack")
        (set `self.IsAttacking` true)
        (`Actor.K2_SetActorRotation` _enemycharacter (`KismetMathLibrary.FindLookAtRotation` (`Actor.K2_GetActorLocation` _enemycharacter) (`Actor.K2_GetActorLocation` _targetcharacter)) false)
        (`|PlayMontage` (`Character.Mesh` _enemycharacter) "/Game/CustomContents/Animation/EnemyAnimations/AM_DualWeaponCombo.AM_DualWeaponCombo" 1.0 0.0 "None" false
          (:`OnCompleted`
            _)
          (:`OnInterrupted`
            (`KismetSystemLibrary.PrintString` "Montage Interrupted")))
        (`self.SetCurrentState` "NewEnumerator2")
        (set `self.IsAttacking` false))
      (:`else`))))

(fn `CalcDistanceToTarget`
  (bind _targetcharacter (`/Game/CustomContents/Blueprints/Character/Enemy/BP_Enemy.TargetCharacter` (`self.EnemyCharacter`))
    (:`then`
      (bind _output_get (set `self.DistanceToTarget` (`KismetMathLibrary.VSizeXY` (- (`Actor.K2_GetActorLocation` _targetcharacter) (`Actor.K2_GetActorLocation` (`self.EnemyCharacter`))))))
      (`KismetSystemLibrary.PrintString` (`KismetStringLibrary.Conv_DoubleToString` _output_get) true true (struct :`G` 1.0 :`B` 0.044426 :`A` 1.0) 2.0 "2"))
    (:`else`)))

(fn `FollowToTarget`
  (bind _enemycharacter (`self.EnemyCharacter`)
    (:`then`
      (bind _targetcharacter (`/Game/CustomContents/Blueprints/Character/Enemy/BP_Enemy.TargetCharacter` _enemycharacter)
        (:`then`
          (bind _returnvalue (- (`Actor.K2_GetActorLocation` _targetcharacter) (`Actor.K2_GetActorLocation` (`self.EnemyCharacter`))))
          (`Actor.K2_SetActorLocation` (`self.EnemyCharacter`) (+ (`Actor.K2_GetActorLocation` (`self.EnemyCharacter`)) (- _returnvalue (* (`KismetMathLibrary.Normal` _returnvalue) 100.0))) true false))
        (:`else`)))
    (:`else`)))

(fn `GetChaseDirection`
  (returns (ReturnValue :type "Vector Structure"))
  (bind _enemycharacter (`self.EnemyCharacter`))
  (bind _targetcharacter (`/Game/CustomContents/Blueprints/Character/Enemy/BP_Enemy.TargetCharacter` _enemycharacter)
    (:`then`
      (return (`KismetMathLibrary.Normal` (- (`Actor.K2_GetActorLocation` _targetcharacter) (`Actor.K2_GetActorLocation` _enemycharacter)))))
    (:`else`)))

(fn `GetChaseTime`
  (returns (ChaseDuration :type "Float (double-precision)"))
  (bind _enemycharacter (`self.EnemyCharacter`))
  (bind _targetcharacter (`/Game/CustomContents/Blueprints/Character/Enemy/BP_Enemy.TargetCharacter` _enemycharacter)
    (:`then`
      (return (/ (`KismetMathLibrary.VSizeXY` (- (`Actor.K2_GetActorLocation` _targetcharacter) (`Actor.K2_GetActorLocation` _enemycharacter))) (`self.ChaseSpeed`))))
    (:`else`)))

(fn `MovingTowardPlayer`
  (locals (Alpha :type "Float (double-precision)") (DeltaMove :type "Vector Structure") (CurveValue :type "Float (double-precision)"))
  (bind _enemycharacter (`self.EnemyCharacter`))
  ; ChaseDuration 시간 동안 추적
  (if (< (`self.ElapsedTime`) (`self.ChaseDuration`))
    (set `self.ElapsedTime` (+ (`self.ElapsedTime`) (`GameplayStatics.GetWorldDeltaSeconds`)))
    (`Actor.K2_SetActorLocation` _enemycharacter (+ (`Actor.K2_GetActorLocation` _enemycharacter) (* (`self.TargetDirection`) (`self.ChaseSpeed`) (`GameplayStatics.GetWorldDeltaSeconds`))) false false)
    (else
      (`self.SetCurrentState` "NewEnumerator0")
      ; 쫓아갔는데도 MinChaseDistance보다 더 멀면 계속 추적
      (if (and (> (`self.DistanceToTarget`) (`self.MinChaseDistance`)) (< (`self.DistanceToTarget`) (`self.MinChaseDistance`)))
        (`self.SetCurrentState` "NewEnumerator2")))))

(fn `RotateToTarget`
  (bind (_returnvalue_roll _returnvalue_pitch _returnvalue_yaw) (`KismetMathLibrary.BreakRotator` (`Actor.K2_GetActorRotation` (`self.EnemyCharacter`))))
  (bind _enemycharacter (`self.EnemyCharacter`)
    (:`then`
      (bind _targetcharacter (`/Game/CustomContents/Blueprints/Character/Enemy/BP_Enemy.TargetCharacter` _enemycharacter)
        (:`then`
          (bind (_returnvalue_roll_2 _returnvalue_pitch_2 _returnvalue_yaw_2) (`KismetMathLibrary.BreakRotator` (`KismetMathLibrary.Conv_VectorToRotator` (- (`Actor.K2_GetActorLocation` _targetcharacter) (`Actor.K2_GetActorLocation` (`self.EnemyCharacter`))))))
          (`Actor.K2_SetActorRotation` (`self.EnemyCharacter`) (`KismetMathLibrary.MakeRotator` _returnvalue_roll _returnvalue_pitch (`KismetMathLibrary.FInterpTo` _returnvalue_yaw _returnvalue_yaw_2 (`GameplayStatics.GetWorldDeltaSeconds`) 200.0)) false))
        (:`else`)))
    (:`else`)))

(fn `SetCurrentState`
  (params (NewState :type "/Game/CustomContents/Components/EEnemyState Enum" :default "NewEnumerator0"))
  (if (`|EnumInequality` NewState (`self.CurrentState`))
    (bind _output_get (set `self.CurrentState` NewState))
    (switch `/Game/CustomContents/Components/EEnemyState` _output_get
      (:`NewEnumerator2`
        (set `self.ElapsedTime` 0.0)
        (set `self.TargetDirection` (`self.GetChaseDirection`))
        (set `self.ChaseDuration` (`self.GetChaseTime`))
        (`self.SetCurrentState` "NewEnumerator5"))
      (:`NewEnumerator3`
        (`self.DualComboAttack`)))))