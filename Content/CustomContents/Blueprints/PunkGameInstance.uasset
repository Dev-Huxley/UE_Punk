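; Game instance that serves as the central master-data lookup and boss phase store for a boss fight.
; Getters read DataTable rows for boss, player and slave stats, keyed config values, and dialog strings for skills, wins and phase 2 entry.
; Skill dialog maps the attack type to a row name through the TypeString map.
; TickBossPhase advances the phase from zero to one, triggers OnBattleMode on BP_Enemy, and reports whether it changed.
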(fn `GetBossPhase`
  (returns (Phase :type Integer))
  (return (`self.BossPhase`)))

(fn `GetBossSkillDialog`
  (params (AttackType :type "/Game/CustomContents/Components/EEnemyAttackType Enum" :default "NewEnumerator8"))
  (returns (Dialog :type String))
  (locals (TypeString :type "Map of /Game/CustomContents/Components/EEnemyAttackType Enum to Name"))
  (bind _returnvalue (`|GetDataTableRow` "/Game/CustomContents/MasterData/MasterData_-_GameStringData.MasterData_-_GameStringData" (`BlueprintMapLibrary.Map_Find` (`local.TypeString`) AttackType))
    (:`then`
      (return (`.Dialog_2_5ABFF8684C3E5D489E60E7A60FE132F4` (break `/Game/CustomContents/MasterData/GameStringData` _returnvalue))))))

(fn `GetBossStat`
  (returns (StatData :type "/Game/CustomContents/MasterData/BossStatData Structure"))
  (bind _returnvalue (`|GetDataTableRow` "/Game/CustomContents/MasterData/MasterData_-_BossStatData.MasterData_-_BossStatData" "Boss")
    (:`then`
      (return _returnvalue))))

(fn `GetBossWinDialog`
  (returns (Dialog :type String))
  (bind _returnvalue (`|GetDataTableRow` "/Game/CustomContents/MasterData/MasterData_-_GameStringData.MasterData_-_GameStringData" "10")
    (:`then`
      (return (`.Dialog_2_5ABFF8684C3E5D489E60E7A60FE132F4` (break `/Game/CustomContents/MasterData/GameStringData` _returnvalue))))))

(fn `GetConfigData`
  (params (Key :type Name))
  (returns (Value :type "Float (double-precision)"))
  (bind _returnvalue (`|GetDataTableRow` "/Game/CustomContents/MasterData/MasterData_-_ConfigData.MasterData_-_ConfigData" Key)
    (:`then`
      (return (break `/Game/CustomContents/MasterData/ConfigData` _returnvalue)))))

(fn `GetPhase2EnterDialog`
  (returns (Dialog :type String))
  (bind _returnvalue (`|GetDataTableRow` "/Game/CustomContents/MasterData/MasterData_-_GameStringData.MasterData_-_GameStringData" "11")
    (:`then`
      (return (`.Dialog_2_5ABFF8684C3E5D489E60E7A60FE132F4` (break `/Game/CustomContents/MasterData/GameStringData` _returnvalue))))))

(fn `GetPlayerStat`
  (returns (StatData :type "/Game/CustomContents/MasterData/PlayerStatData Structure"))
  (bind _returnvalue (`|GetDataTableRow` "/Game/CustomContents/MasterData/MasterData_-_PlayerStatData.MasterData_-_PlayerStatData" "Player")
    (:`then`
      (return _returnvalue))))

(fn `GetPlayerWinDialog`
  (returns (Dialog :type String))
  (bind _returnvalue (`|GetDataTableRow` "/Game/CustomContents/MasterData/MasterData_-_GameStringData.MasterData_-_GameStringData" "9")
    (:`then`
      (return (`.Dialog_2_5ABFF8684C3E5D489E60E7A60FE132F4` (break `/Game/CustomContents/MasterData/GameStringData` _returnvalue))))))

(fn `GetSlaveStat`
  (returns (StatData :type "/Game/CustomContents/MasterData/SlaveStatData Structure"))
  (bind _returnvalue (`|GetDataTableRow` "/Game/CustomContents/MasterData/MasterData_-_SlaveStatData.MasterData_-_SlaveStatData" "Slave")
    (:`then`
      (return _returnvalue))))

(fn `TickBossPhase`
  (returns (Change :type Boolean))
  (if (== (`self.BossPhase`) 0)
    (set `self.BossPhase` 1)
    (`|ExecutionSequence`
      (:`then_0`
        (bind _returnvalue (`GameplayStatics.GetActorOfClass` "/Game/CustomContents/Blueprints/Character/Enemy/BP_Enemy.BP_Enemy_C"))
        (`/Game/CustomContents/Blueprints/Character/Enemy/BP_Enemy.OnBattleMode` _returnvalue))
      (:`then_1`
        (return true)))
    (else
      (return false))))

(fn `UpdateBossPhase`
  (params (Phase :type Integer))
  (set `self.BossPhase` Phase))