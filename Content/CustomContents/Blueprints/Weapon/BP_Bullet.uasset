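; BP_Bullet is a weapon bullet actor that damages BP_Enemy actors it hits.
; When its Sphere overlaps an actor that casts to BP_Enemy, it applies random damage, spawns an emitter at its own location and destroys itself.
; Other actors are ignored, and a short BeginPlay delay serves as its lifetime, after which it also spawns an emitter and is destroyed.
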(event `self.ReceiveBeginPlay`
  ; 총알 생성 후 2.5초 destroy
  (`KismetSystemLibrary.Delay` 2.5)
  (`GameplayStatics.SpawnEmitterAtLocation` null)
  (`self.K2_DestroyActor`))

(event `self.Sphere.OnComponentBeginOverlap`
  (params (OverlappedComponent :type "PrimitiveComponent Object Reference") (OtherActor :type "Actor Object Reference") (OtherComp :type "PrimitiveComponent Object Reference") (OtherBodyIndex :type Integer) (bFromSweep :type Boolean) (SweepResult :type "HitResult Structure (by ref)"))
  ; Enemy태그 체크하고 맞다면 destroy+emitter
  (bind _asbp_enemy (cast `/Game/CustomContents/Blueprints/Character/Enemy/BP_Enemy` OtherActor))
  (bind _output_get (set `self.Damage` (`KismetMathLibrary.RandomFloatInRange` 5.0 10.0)))
  (`GameplayStatics.ApplyDamage` _asbp_enemy _output_get null self)
  (`GameplayStatics.SpawnEmitterAtLocation` null (`self.K2_GetActorLocation`))
  (`self.K2_DestroyActor`))

(fn `UserConstructionScript`)