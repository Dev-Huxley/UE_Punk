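; Enemy character Blueprint that handles player detection, melee attacks and damage reactions.
; TempDetector overlap passes the player to AIC_Enemy as target, and BPCStatSystem applies incoming damage using the HUD widget.
; Hit and death states feed the Blackboard, triggering knockback with a random hit montage, or a death montage and delayed destroy.
; StartAttack schedules a right-arm sphere trace via short timer, damaging actors tagged Player.
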(event `self.ReceiveBeginPlay`
  ; Begin-Set Animation BP
  (bind _asabp_enemy (cast `/Game/CustomContents/Blueprints/ABP_Enemy` (`SkeletalMeshComponent.GetAnimInstance` (`self.Mesh`))))
  (set `self.AnimationBP` _asabp_enemy)
  ; Set WB_HUD
  (bind _aswb_hud (cast `/Game/CustomContents/UI/WB_HUD` (`WidgetComponent.GetUserWidgetObject` (`self.HUD`))))
  (set `self.WB HUD` _aswb_hud))

(event `self.TempDetector.OnComponentBeginOverlap`
  (params (OverlappedComponent :type "PrimitiveComponent Object Reference") (OtherActor :type "Actor Object Reference") (OtherComp :type "PrimitiveComponent Object Reference") (OtherBodyIndex :type Integer) (bFromSweep :type Boolean) (SweepResult :type "HitResult Structure (by ref)"))
  ; OnBegin(TmpDector)
  (bind _asbp_player_character (cast `/Game/CustomContents/Blueprints/BP_PlayerCharacter` OtherActor))
  (bind _asaic_enemy (cast `/Game/CustomContents/Blueprints/AIC_Enemy` (`AIBlueprintHelperLibrary.GetAIController` self)))
  (`/Game/CustomContents/Blueprints/AIC_Enemy.Set Target` _asaic_enemy _asbp_player_character))

(event `self.ReceiveAnyDamage`
  (params (Damage :type "Float (single-precision)") (DamageType :type "DamageType Object Reference") (InstigatedBy :type "Controller Object Reference") (DamageCauser :type "Actor Object Reference"))
  ; OnDamaged
  (bind _output_get (set `self.IsHit` true))
  ;;[0.15 0.000275 0.1462 0.5] SetBlackBoardValue
  (`BlackboardComponent.SetValueAsBool` (`AIBlueprintHelperLibrary.GetBlackboard` null) (`self.IsHitBlackboardKey`) _output_get)
  (set `self.Damage Causer` DamageCauser)
  (bind _isdead (`/Game/CustomContents/Components/BPC_StatSystem.DecreaseHealth` (`self.BPC_StatSystem`) Damage (`self.WB HUD`)))
  (bind _output_get_2 (set `self.Is Dead` _isdead))
  (if _output_get_2
    ; OnDead
    ;;[0.01847 0 0.15 0.5] SetBlackboardValue
    (`BlackboardComponent.SetValueAsBool` (`AIBlueprintHelperLibrary.GetBlackboard` null) (`self.IsDeadBlackboardKey`) (`self.Is Dead`))
    (`self.PlayAnimMontage` "/Game/CustomContents/Animation/Montages/Death_Montage.Death_Montage") ; 사망 애니메이션 재생
    ;;[0.15 0.02547 9.4e-05 0.5] 사망시 처리, 콜리전을 Off후,  5초후 액터 제거
    (`PrimitiveComponent.SetCollisionEnabled` (`self.CapsuleComponent`) "NoCollision")
    (`KismetSystemLibrary.Delay` 5.0)
    (`self.K2_DestroyActor`)
    (else
      ; OnHit
      (`self.SetBackEnemyLocation` (`self.Damage Causer`) 20.0) ; Hit시 DamageCauser방향으로 이동
      (bind _delaytime (`self.Play Hit Animation` (`self.HitMontages`))) ; 피격 애니메이션 재생
      ; HitEnd
      (`KismetSystemLibrary.Delay` _delaytime)
      (set `self.IsHit` false)
      (`BlackboardComponent.SetValueAsBool` (`AIBlueprintHelperLibrary.GetBlackboard` null) (`self.IsHitBlackboardKey`) false))))

(event `StartAttack`
  ; OnStartAttack
  (bind _returnvalue (`KismetSystemLibrary.K2_SetTimerDelegate` (delegate `Attack`) 0.01))
  (set `self.AttackTimerHandler` _returnvalue))

(event `StopAttack`
  ; OnStopAttack
  (`KismetSystemLibrary.K2_ClearAndInvalidateTimerHandle` (`self.AttackTimerHandler`)))

(event `Attack`
  ; OnAttack
  (bind (_outhit _returnvalue) (`KismetSystemLibrary.SphereTraceSingle` :`Start` (`SceneComponent.K2_GetComponentLocation` (`self.RightArmStart`)) :`End` (`SceneComponent.K2_GetComponentLocation` (`self.RightArmEnd`)) :`Radius` 50.0 :`TraceChannel` "TraceTypeQuery1" :`DrawDebugType` "ForDuration" :`TraceHitColor` (struct :`R` 1.0 :`G` 0.327897 :`A` 1.0) :`DrawTime` 7.0))
  (if _returnvalue
    (bind (_bblockinghit _binitialoverlap _time _distance _location _impactpoint _normal _impactnormal _physmat _hitactor) (`GameplayStatics.BreakHitResult` _outhit))
    (if (`self.ActorHasTag` _hitactor "Player")
      (`GameplayStatics.ApplyDamage` _hitactor 20.0 null self)
      (else
        (`KismetSystemLibrary.PrintString` "Not Player Hit")))
    (else
      (`KismetSystemLibrary.PrintString` "EnemyAttack Failed!"))))

(fn `Play Hit Animation`
  (params (Array :type "Array of AnimMontage Object Reference"))
  (returns (DelayTime :type "Float (single-precision)"))
  (bind _returnvalue (`self.PlayAnimMontage` (`|GetArrayItem` Array (`KismetMathLibrary.RandomIntegerInRange` 0 (- (`KismetArrayLibrary.Array_Length` Array) 1)))))
  (return _returnvalue))

(fn `SetBackEnemyLocation`
  (params (`Damage Causer` :type "Actor Object Reference") (`Back Value` :type "Float (double-precision)"))
  (`self.K2_SetActorLocation` (+ (* (`self.GetActorForwardVector` `Damage Causer`) `Back Value`) (`self.K2_GetActorLocation`))))

(fn `UserConstructionScript`)