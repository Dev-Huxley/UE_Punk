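; Object pool actor for Demolitionist Gunner fire-shot projectiles, pre-spawning a hidden, collision-disabled batch on BeginPlay.
; GetPool is meant to reuse an idle projectile, but its inverted Find check skips every entry, so it always spawns, stores and returns a new active one.
; ReturnPool hides a projectile and disables its collision, without clearing its InUse flag.
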(event `self.ReceiveBeginPlay`
  (for _ (range 21)
    (bind _returnvalue (`|SpawnActorFromClass` "/Game/POLYMORPHFX/DemolitionistGunnerFireShotVFX/Blueprints/BP_Demolitionist_Gunner_FireShot_Projectile_01.BP_Demolitionist_Gunner_FireShot_Projectile_01_C" (`self.GetTransform`) "Undefined" "MultiplyWithRoot" null null))
    (`self.SetActorHiddenInGame` _returnvalue true)
    (`self.SetActorEnableCollision` _returnvalue false)
    (`KismetArrayLibrary.Array_Add` (`self.ObjectPoool`) _returnvalue)
    (`KismetSystemLibrary.PrintString` (`KismetStringLibrary.Conv_IntToString` (`KismetArrayLibrary.Array_Length` (`self.ObjectPoool`))))))

(fn `GetPool`
  (returns (Return :type "/Game/POLYMORPHFX/DemolitionistGunnerFireShotVFX/Blueprints/BP_Demolitionist_Gunner_FireShot_Projectile_01 Object Reference"))
  (locals (Find :type Boolean))
  (set `local.Find` false)
  (for _array_element (`self.ObjectPoool`)
    (if (== (`local.Find`) false)
      _
      (elif (== (`/Game/POLYMORPHFX/DemolitionistGunnerFireShotVFX/Blueprints/BP_Demolitionist_Gunner_FireShot_Projectile_01.InUse` _array_element) false)
        (`|ExecutionSequence`
          (:`then_0`
            (`self.SetActorEnableCollision` _array_element true))
          (:`then_1`
            (`self.SetActorHiddenInGame` _array_element false))
          (:`then_2`
            (set `/Game/POLYMORPHFX/DemolitionistGunnerFireShotVFX/Blueprints/BP_Demolitionist_Gunner_FireShot_Projectile_01.InUse` true _array_element))
          (:`then_3`
            (set `local.Find` true))
          (:`then_4`
            (return _array_element))))))
  (if (== (`local.Find`) false)
    (bind _returnvalue (`|SpawnActorFromClass` "/Game/POLYMORPHFX/DemolitionistGunnerFireShotVFX/Blueprints/BP_Demolitionist_Gunner_FireShot_Projectile_01.BP_Demolitionist_Gunner_FireShot_Projectile_01_C" (`self.GetTransform`) "Undefined" "MultiplyWithRoot" null null))
    (`self.SetActorHiddenInGame` _returnvalue false)
    (`self.SetActorEnableCollision` _returnvalue true)
    (set `/Game/POLYMORPHFX/DemolitionistGunnerFireShotVFX/Blueprints/BP_Demolitionist_Gunner_FireShot_Projectile_01.InUse` false _returnvalue)
    (`KismetArrayLibrary.Array_Add` (`self.ObjectPoool`) _returnvalue)
    (return _returnvalue)))

(fn `ReturnPool`
  (params (ReturnObject :type "/Game/POLYMORPHFX/DemolitionistGunnerFireShotVFX/Blueprints/BP_Demolitionist_Gunner_FireShot_Projectile_01 Object Reference"))
  (`self.SetActorHiddenInGame` ReturnObject true)
  (`self.SetActorEnableCollision` ReturnObject false))

(fn `UserConstructionScript`)