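; Enemy character Blueprint for a dual-sword melee foe that hands a detected player to its AI controller as target.
; Damage updates health and blackboard flags, then triggers random hit montages with knockback, or death and delayed destruction.
; Attack events run sphere traces along the selected sword to damage the player; a dash attack launches it forward between montages.
; Slow-motion ("Sandevistan") events scale montage rates, dash velocity and walk speed.
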(event `self.ReceiveBeginPlay`
  ; Begin-Set Animation BP
  (bind _asabp_enemy (cast `/Game/CustomContents/Blueprints/Character/Enemy/ABP_Enemy` (`SkeletalMeshComponent.GetAnimInstance` (`self.Mesh`))))
  (set `self.AnimationBP` _asabp_enemy)
  (`self.SetUpWeaponCollision`))

(event `self.TempDetector.OnComponentBeginOverlap`
  (params (OverlappedComponent :type "PrimitiveComponent Object Reference") (OtherActor :type "Actor Object Reference") (OtherComp :type "PrimitiveComponent Object Reference") (OtherBodyIndex :type Integer) (bFromSweep :type Boolean) (SweepResult :type "HitResult Structure (by ref)"))
  ; OnBegin(TmpDector)
  (bind _asbp_player_character (cast `/Game/CustomContents/Blueprints/Character/Player/BP_PlayerCharacter` OtherActor))
  (bind _asaic_enemy (cast `/Game/CustomContents/Blueprints/AI/AIC_Enemy` (`AIBlueprintHelperLibrary.GetAIController` self)))
  (`/Game/CustomContents/Blueprints/AI/AIC_Enemy.Set Target` _asaic_enemy _asbp_player_character))

(event `self.ReceiveAnyDamage`
  (params (Damage :type "Float (single-precision)") (DamageType :type "DamageType Object Reference") (InstigatedBy :type "Controller Object Reference") (DamageCauser :type "Actor Object Reference"))
  ; OnDamaged
  (bind _output_get (set `self.IsHit` true))
  ;;[0.15 0.000275 0.1462 0.5] SetBlackBoardValue
  (`BlackboardComponent.SetValueAsBool` (`AIBlueprintHelperLibrary.GetBlackboard` null) (`self.IsHitBlackboardKey`) _output_get)
  (set `self.Damage Causer` DamageCauser)
  ; DecreaseHealth
  (bind _aswb_hud (cast `/Game/CustomContents/UI/WB_HUD` (`WidgetComponent.GetUserWidgetObject` (`self.Widget`))))
  (bind _isdead (`/Game/CustomContents/Components/BPC_StatSystem.DecreaseHealth` (`self.BPC_StatSystem`) Damage _aswb_hud))
  (bind _output_get_2 (set `self.Is Dead` _isdead))
  (if _output_get_2
    ;[0.15 0.03234 0.04202 0.5] OnDead
    ;;[0.01847 0 0.15 0.5] SetBlackboardValue
    (`BlackboardComponent.SetValueAsBool` (`AIBlueprintHelperLibrary.GetBlackboard` null) (`self.IsDeadBlackboardKey`) (`self.Is Dead`))
    (`self.PlayAnimMontage` "/Game/CustomContents/Animation/Montages/Death_Montage.Death_Montage" (`self.SlowSpeed`)) ; 사망 애니메이션 재생
    ;;[0.15 0.02547 9.4e-05 0.5] 사망시 처리, 콜리전을 Off후,  5초후 액터 제거
    (`PrimitiveComponent.SetCollisionEnabled` (`self.CapsuleComponent`) "NoCollision")
    (`KismetSystemLibrary.Delay` 5.0)
    (`self.K2_DestroyActor`)
    (else
      ; OnHit
      (`self.SetBackEnemyLocation` (`self.Damage Causer`) 20.0) ; Hit시 DamageCauser방향으로 이동
      (bind _delaytime (`self.Play Hit Animation` (`self.HitMontages`))) ; 피격 애니메이션 재생
      ; HitEnd
      (`KismetSystemLibrary.Delay` _delaytime)
      (set `self.IsHit` false)
      (`BlackboardComponent.SetValueAsBool` (`AIBlueprintHelperLibrary.GetBlackboard` null) (`self.IsHitBlackboardKey`) false))))

(event `StartAttack`
  ; OnStartAttack
  (bind _returnvalue (`KismetSystemLibrary.K2_SetTimerDelegate` (delegate `Attack`) 0.01))
  (set `self.AttackTimerHandler` _returnvalue))

(event `StopAttack`
  ; OnStopAttack
  (`KismetSystemLibrary.K2_ClearAndInvalidateTimerHandle` (`self.AttackTimerHandler`)))

(event `DashAttack`
  ; Dash Attack
  (`KismetSystemLibrary.PrintString` "Dash")
  (`|PlayMontage` (`self.Mesh`) "/Game/CustomContents/Animation/AttackAnimations/AM_DashAttackReady.AM_DashAttackReady" (`self.SlowSpeed`)
    (:`OnCompleted`
      (set `CharacterMovementComponent.GravityScale` 0.3 (`self.CharacterMovement`))
      (`self.LaunchCharacter` (* (`self.GetActorForwardVector`) (* (`self.SlowSpeed`) 4000.0)))
      (`KismetSystemLibrary.Delay` 0.1)
      (`|PlayMontage` (`self.Mesh`) "/Game/CustomContents/Animation/EnemyAnimations/AM_DashAttack.AM_DashAttack" (`self.SlowSpeed`)
        (:`OnCompleted`
          (set `CharacterMovementComponent.GravityScale` 1.0 (`self.CharacterMovement`)))))))

(event `Attack`
  ; OnAttack
  (`self.TraceToAttack` (`self.TraceStartLoc`) (`self.TraceEndLoc`)))

(event `SetLeftSwordTraceLoc`
  ; SetLeftSwordTraceLocation
  (set `self.TraceStartLoc` (`self.GetTraceLocStart` (`self.LeftSwordRef`)))
  (set `self.TraceEndLoc` (`self.GetTraceLocEnd` (`self.LeftSwordRef`))))

(event `SetRightSwordTraceLoc`
  ; SetRightSwordTraceLocation
  (set `self.TraceStartLoc` (`self.GetTraceLocStart` (`self.RightSwordRef`)))
  (set `self.TraceEndLoc` (`self.GetTraceLocEnd` (`self.RightSwordRef`))))

(event `self.EnterSlowMotion`
  ; Enter Slow Motion
  (set `self.SlowSpeed` 0.3)
  (set `CharacterMovementComponent.MaxWalkSpeed` 30.0 (`self.CharacterMovement`))
  (`KismetSystemLibrary.PrintString` "Enter Sandevistan"))

(event `self.ExitSlowMotion`
  ; Exit Slow Motion
  (set `self.SlowSpeed` 1.0)
  (set `CharacterMovementComponent.MaxWalkSpeed` 100.0 (`self.CharacterMovement`))
  (`KismetSystemLibrary.PrintString` "Exit Sandevistan"))

(fn `GetTraceLocEnd`
  (params (Ref :type "/Game/CustomContents/Blueprints/Actor/BP_Sword Object Reference"))
  (returns (Location :type "Vector Structure"))
  (return (`SceneComponent.K2_GetComponentLocation` (`/Game/CustomContents/Blueprints/Actor/BP_Sword.TraceEnd` Ref))))

(fn `GetTraceLocStart`
  (params (Ref :type "/Game/CustomContents/Blueprints/Actor/BP_Sword Object Reference"))
  (returns (Location :type "Vector Structure"))
  (return (`SceneComponent.K2_GetComponentLocation` (`/Game/CustomContents/Blueprints/Actor/BP_Sword.TraceStart` Ref))))

(fn `Play Hit Animation`
  (params (Array :type "Array of AnimMontage Object Reference"))
  (returns (DelayTime :type "Float (single-precision)"))
  (bind _returnvalue (`self.PlayAnimMontage` (`|GetArrayItem` Array (`KismetMathLibrary.RandomIntegerInRange` 0 (- (`KismetArrayLibrary.Array_Length` Array) 1))) (`self.SlowSpeed`)))
  (return _returnvalue))

(fn `SetBackEnemyLocation`
  (params (`Damage Causer` :type "Actor Object Reference") (`Back Value` :type "Float (double-precision)"))
  (`self.K2_SetActorLocation` (+ (* (`self.GetActorForwardVector` `Damage Causer`) `Back Value`) (`self.K2_GetActorLocation`))))

(fn `SetUpWeaponCollision`
  (bind _asbp_sword (cast `/Game/CustomContents/Blueprints/Actor/BP_Sword` (`ChildActorComponent.ChildActor` (`self.LeftSword`))))
  (bind _output_get (set `self.LeftSwordRef` _asbp_sword))
  (`self.SetOwner` _output_get self)
  (bind _asbp_sword_2 (cast `/Game/CustomContents/Blueprints/Actor/BP_Sword` (`ChildActorComponent.ChildActor` (`self.RightSword`))))
  (bind _output_get_2 (set `self.RightSwordRef` _asbp_sword_2))
  (`self.SetOwner` _output_get_2 self)
  (`PrimitiveComponent.IgnoreActorWhenMoving` (`/Game/CustomContents/Blueprints/Actor/BP_Sword.Box` (`self.LeftSwordRef`)) (`self.RightSwordRef`) true)
  (`PrimitiveComponent.IgnoreActorWhenMoving` (`/Game/CustomContents/Blueprints/Actor/BP_Sword.Box` (`self.RightSwordRef`)) (`self.RightSwordRef`) true)
  (`PrimitiveComponent.IgnoreActorWhenMoving` (`/Game/CustomContents/Blueprints/Actor/BP_Sword.Box` (`self.LeftSwordRef`)) self true)
  (`PrimitiveComponent.IgnoreActorWhenMoving` (`/Game/CustomContents/Blueprints/Actor/BP_Sword.Box` (`self.RightSwordRef`)) self true))

(fn `TraceToAttack`
  (params (TraceStartLocation :type "Vector Structure") (TraceEndLocation :type "Vector Structure"))
  (bind (_outhit _returnvalue) (`KismetSystemLibrary.SphereTraceSingle` :`Start` TraceStartLocation :`End` TraceEndLocation :`Radius` 50.0 :`TraceChannel` "TraceTypeQuery1" :`DrawDebugType` "ForDuration" :`TraceHitColor` (struct :`R` 1.0 :`G` 0.327897 :`A` 1.0) :`DrawTime` 7.0))
  (if _returnvalue
    (bind (_bblockinghit _binitialoverlap _time _distance _location _impactpoint _normal _impactnormal _physmat _hitactor) (`GameplayStatics.BreakHitResult` _outhit))
    (if (`self.ActorHasTag` _hitactor "Player")
      (`GameplayStatics.ApplyDamage` _hitactor 20.0 null self)
      (else
        (`KismetSystemLibrary.PrintString` "Not Player Hit")))
    (else
      (`KismetSystemLibrary.PrintString` "EnemyAttack Failed!"))))

(fn `UserConstructionScript`)