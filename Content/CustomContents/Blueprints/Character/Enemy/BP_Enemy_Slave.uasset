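; BP_Enemy_Slave is an enemy Blueprint that keeps a motion warp target aligned to the player.
; A temporary detector component stores any overlapping BP_PlayerCharacter as TargetCharacter, with no logic to clear it.
; While that target is valid, Tick updates the "Warp" target on MotionWarping to a point in front of the player, using the player's rotation.
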(event `self.TempDetector.OnComponentBeginOverlap`
  (params (OverlappedComponent :type "PrimitiveComponent Object Reference") (OtherActor :type "Actor Object Reference") (OtherComp :type "PrimitiveComponent Object Reference") (OtherBodyIndex :type Integer) (bFromSweep :type Boolean) (SweepResult :type "HitResult Structure (by ref)"))
  ; OnBegin(TmpDector)
  (bind _asbp_player_character (cast `/Game/CustomContents/Blueprints/Character/Player/BP_PlayerCharacter` OtherActor))
  (set `self.TargetCharacter` _asbp_player_character))

(event `self.ReceiveTick`
  (params (DeltaSeconds :type "Float (single-precision)"))
  ; Tick
  (bind _targetcharacter (`self.TargetCharacter`)
    (:`then`
      (bind _motionwarping (`self.MotionWarping`)
        (:`then`
          (`MotionWarpingComponent.AddOrUpdateWarpTarget` _motionwarping (make `MotionWarpingTarget` "Warp" (+ (`self.K2_GetActorLocation` _targetcharacter) (* (`self.GetActorForwardVector` _targetcharacter) 200.0)) (`self.K2_GetActorRotation` _targetcharacter) null "None")))
        (:`else`)))
    (:`else`)))

(fn `UserConstructionScript`
  (`parent.UserConstructionScript`))