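; Player character Blueprint with Enhanced Input movement, first/third-person camera switching and Fist/Sword/Gun cycling that reuses spawned weapons.
; Stat and attack components supply health, ammo and aim detection, which feed the UI component.
; OnDamage drives hit reactions or death, game-over UI and actor destruction, while AnyDamage is deprecated.
; Skills include trace-targeted homing bullet volleys and Sandevistan, a cooldown-gated global slow motion that offsets the player's own time dilation.
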(event `self.ReceiveBeginPlay`
  ; InitDebugState
  (bind _debugenable (`/Game/CustomContents/UI/BP/BPC_UserInterface.DebugDraw` (`self.BPC_UserInterface`)))
  (set `self.Debug Enable` _debugenable)
  ; InitMinimap
  (`PrimitiveComponent.SetHiddenInSceneCapture` (`self.Mesh`) true)
  ;[0 0.15 0.008756 0.5] Begin-EnhancedInputAction
  (bind _asplayer_controller (cast `PlayerController` (`self.GetController`)))
  (message `EnhancedInputSubsystemInterface.AddMappingContext` (pcsubsystem `EnhancedInputLocalPlayerSubsystem` _asplayer_controller) "/Game/CustomContents/Input/IMC_Player.IMC_Player" 0 (struct))
  ;[0.07019 0.15 0.01246 0.5] InitPlayerUI
  (`self.UpdatePlayerHealthDisplay`)
  (`/Game/CustomContents/UI/BP/BPC_UserInterface.OnAim` (`self.BPC_UserInterface`) false)
  (`/Game/CustomContents/UI/BP/BPC_UserInterface.OnWeaponChange` (`self.BPC_UserInterface`) (`self.CurrentWeaponType`))
  ; InitBullet
  (`/Game/CustomContents/UI/BP/BPC_UserInterface.OnUpdateEquipBullet` (`self.BPC_UserInterface`) (`/Game/CustomContents/Components/BPC_PlayerStatSystem.EquipBullet` (`self.BPC_PlayerStatSystem`)))
  (`/Game/CustomContents/UI/BP/BPC_UserInterface.OnUpdateHasBullet` (`self.BPC_UserInterface`) (`/Game/CustomContents/Components/BPC_PlayerStatSystem.HasBullet` (`self.BPC_PlayerStatSystem`))))

(event `self.ReceiveTick`
  (params (DeltaSeconds :type "Float (single-precision)"))
  ;[0.15 0.1247 0 0.5] Tick
  (set `self.SandevistanCnt` (+ (`GameplayStatics.GetWorldDeltaSeconds`) (`self.SandevistanCnt`)))
  ;[1 0.3279 0] Aim
  (bind (_detect _enemy) (`/Game/CustomContents/Components/BPC_AttackSystem.DetectLookAtTarget` (`self.BPC_AttackSystem`) 1000.0 16.0))
  (`/Game/CustomContents/UI/BP/BPC_UserInterface.OnAim` (`self.BPC_UserInterface`) _detect)
  ; OnAimTarget
  (`/Engine/EditorBlueprintResources/StandardMacros.IsValid` null
    (:`Is Valid`
      (`/Game/CustomContents/Blueprints/Character/Enemy/BP_Enemy.OnAimTarget` _enemy _detect) ; 에임 대상인 타겟의 체력바 정리
    )))

(event `self.ReceiveAnyDamage`
  (params (Damage :type "Float (single-precision)") (DamageType :type "DamageType Object Reference") (InstigatedBy :type "Controller Object Reference") (DamageCauser :type "Actor Object Reference"))
  ;[0.15 0 0.007219 0.5] DamageProcess
  (`KismetSystemLibrary.PrintString` "Deprecated Play ApplyDamage"))

(event `OnDamage`
  (params (Damage :type "Float (double-precision)") (Critical :type Boolean) (`Instigated By` :type "Controller Object Reference") (`Damage Causer` :type "Actor Object Reference"))
  ;[0.15 0 0.007219 0.5] DamageProcess
  ;;[0.15 0 0.02095 0.5] OnDamaged
  (set `self.IsHitting` true)
  ;; DecreaseHealth
  (bind _isdead (`/Game/CustomContents/Components/BPC_PlayerStatSystem.DecreaseHealth` (`self.BPC_PlayerStatSystem`) Damage))
  (`/Game/CustomContents/UI/BP/BPC_UserInterface.SetCause` (`self.BPC_UserInterface`) `Damage Causer`)
  (`self.UpdatePlayerHealthDisplay`)
  (bind _output_get (set `self.IsDead` _isdead))
  (if _output_get
    ;; OnDead
    (set `CameraComponent.bUsePawnControlRotation` false (`self.FirstPersonCamera`))
    (`self.PlayAnimMontage` "/Game/CustomContents/Animation/Montages/Death_Montage.Death_Montage") ; 사망 애니메이션 재생
    ;;;[0.15 0.02547 9.4e-05 0.5] 사망시 처리, 콜리전을 Off후,  5초후 액터 제거
    (`PrimitiveComponent.SetCollisionEnabled` (`self.CapsuleComponent`) "NoCollision")
    (`self.OnPlayerDied`)
    (`KismetSystemLibrary.Delay` 5.0)
    ;[0.15 0.03048 0 0.5] GameOver
    (`/Game/CustomContents/UI/BP/BP_UI.UpdateCombatState` (`/Game/CustomContents/UI/BP/BPC_UserInterface.BP UI` (`self.BPC_UserInterface`)) "NewEnumerator2")
    (`self.K2_DestroyActor`)
    (else
      ;; Hit
      (`|PlayMontage` (`self.Mesh`) "/Game/CustomContents/Animation/Montages/Hit_1_Montage.Hit_1_Montage"
        (:`then`
          (set `self.IsHitting` false))))))

(event `EnhancedInput|/Game/CustomContents/Input/IA_LookAround`
  (params (ActionValue :type "Vector2D Structure") (ElapsedSeconds :type "Float (double-precision)") (TriggeredSeconds :type "Float (double-precision)") (InputAction :type "InputAction Object Reference" :default "/Game/CustomContents/Input/IA_LookAround.IA_LookAround"))
  ;[0.04097 0 0.15 0.5] OnInputAction
  ;; OnInputAction_LookAround
  (:`Triggered`
    (`self.AddControllerYawInput` ActionValue_X)
    (`self.AddControllerPitchInput` ActionValue_Y)))

(event `EnhancedInput|/Game/CustomContents/Input/IA_JumpCustom`
  (params (ActionValue :type Boolean) (ElapsedSeconds :type "Float (double-precision)") (TriggeredSeconds :type "Float (double-precision)") (InputAction :type "InputAction Object Reference" :default "/Game/CustomContents/Input/IA_JumpCustom.IA_JumpCustom"))
  ;[0.04097 0 0.15 0.5] OnInputAction
  ;; OnInputAction_Jump
  (:`Started`
    (`self.Jump`))
  (:`Completed`
    (`self.StopJumping`)))

(event `EnhancedInput|/Game/CustomContents/Input/IA_Pause`
  (params (ActionValue :type Boolean) (ElapsedSeconds :type "Float (double-precision)") (TriggeredSeconds :type "Float (double-precision)") (InputAction :type "InputAction Object Reference" :default "/Game/CustomContents/Input/IA_Pause.IA_Pause"))
  ;[0.04097 0 0.15 0.5] OnInputAction
  ;; OnInputAction_Pause
  (:`Started`
    (`/Game/CustomContents/UI/BP/BPC_UserInterface.OnPause` (`self.BPC_UserInterface`))))

(event `EnhancedInput|/Game/CustomContents/Input/IA_Movement`
  (params (ActionValue :type "Vector2D Structure") (ElapsedSeconds :type "Float (double-precision)") (TriggeredSeconds :type "Float (double-precision)") (InputAction :type "InputAction Object Reference" :default "/Game/CustomContents/Input/IA_Movement.IA_Movement"))
  (bind (_returnvalue_roll _returnvalue_pitch _returnvalue_yaw) (`KismetMathLibrary.BreakRotator` (`self.GetControlRotation`)))
  (bind (_returnvalue_roll_2 _returnvalue_pitch_2 _returnvalue_yaw_2) (`KismetMathLibrary.BreakRotator` (`self.GetControlRotation`)))
  ;[0.04097 0 0.15 0.5] OnInputAction
  ;; OnInputAction_Movement
  (:`Triggered`
    (if (not (`self.IsHitting`))
      (`self.AddMovementInput` (`KismetMathLibrary.GetRightVector` (`KismetMathLibrary.MakeRotator` _returnvalue_roll_2 0.0 _returnvalue_yaw_2)) ActionValue_X)
      (`self.AddMovementInput` (`KismetMathLibrary.GetForwardVector` (`KismetMathLibrary.MakeRotator` 0.0 0.0 _returnvalue_yaw)) ActionValue_Y))))

(event `EnhancedInput|/Game/CustomContents/Input/IA_WeaponSwitching`
  (params (ActionValue :type Boolean) (ElapsedSeconds :type "Float (double-precision)") (TriggeredSeconds :type "Float (double-precision)") (InputAction :type "InputAction Object Reference" :default "/Game/CustomContents/Input/IA_WeaponSwitching.IA_WeaponSwitching"))
  ;[0.15 0.03732 0 0.5] 장비 전환
  (:`Triggered`
    (switch `/Game/CustomContents/Blueprints/EWeaponType` (`self.CurrentWeaponType`)
      (:`NewEnumerator0`
        (set `self.CurrentWeaponType` "NewEnumerator2")
        (`/Engine/EditorBlueprintResources/StandardMacros.IsValid` (`self.LeftSwordRef`)
          (:`Is Valid`
            (`self.K2_AttachToComponent` (`self.LeftSwordRef`) (`self.Mesh`) "LeftHandWeaponSocket" "KeepRelative" "KeepRelative" "KeepRelative" true)
            (`self.K2_AttachToComponent` (`self.RightSwordRef`) (`self.Mesh`) "RightHandWeaponSocket" "KeepRelative" "KeepRelative" "KeepRelative" true))
          (:`Is Not Valid`
            (bind _returnvalue (`self.SpawnWeaponAndAttach` "/Game/CustomContents/Blueprints/Weapon/BP_Sword.BP_Sword_C" (`self.LeftHandWeaponSocketName`)))
            (set `self.LeftSwordRef` _returnvalue)
            (bind _returnvalue_2 (`self.SpawnWeaponAndAttach` "/Game/CustomContents/Blueprints/Weapon/BP_Sword.BP_Sword_C" (`self.RightHandWeaponSocketName`)))
            (set `self.RightSwordRef` _returnvalue_2))))
      (:`NewEnumerator2`
        (set `self.CurrentWeaponType` "NewEnumerator3")
        (`self.DetachWeapon` (`self.LeftSwordRef`))
        (`self.DetachWeapon` (`self.RightSwordRef`))
        (`/Engine/EditorBlueprintResources/StandardMacros.IsValid` (`self.GunRef`)
          (:`Is Valid`
            (`self.K2_AttachToComponent` (`self.GunRef`) (`self.Mesh`) (`self.GunSocketName`) "KeepRelative" "KeepRelative" "KeepRelative" true))
          (:`Is Not Valid`
            (bind _returnvalue_3 (`self.SpawnWeaponAndAttach` "/Game/CustomContents/Blueprints/Weapon/BP_Gun.BP_Gun_C" (`self.GunSocketName`)))
            (set `self.GunRef` _returnvalue_3))))
      (:`NewEnumerator3`
        (set `self.CurrentWeaponType` "NewEnumerator0")
        (`self.DetachWeapon` (`self.GunRef`))))
    ;[0.4678 0.03793 0.05439] OnWeaponChange
    (`/Game/CustomContents/UI/BP/BPC_UserInterface.OnWeaponChange` (`self.BPC_UserInterface`) (`self.CurrentWeaponType`))))

(event `EnhancedInput|/Game/CustomContents/Input/IA_Crouch`
  (params (ActionValue :type Boolean) (ElapsedSeconds :type "Float (double-precision)") (TriggeredSeconds :type "Float (double-precision)") (InputAction :type "InputAction Object Reference" :default "/Game/CustomContents/Input/IA_Crouch.IA_Crouch"))
  (bind _bpc_userinterface (`self.BPC_UserInterface`))
  ;[0.04097 0 0.15 0.5] OnInputAction
  ;; OnInputAction_Crounch
  (:`Started`
    (`/Engine/EditorBlueprintResources/StandardMacros.FlipFlop`
      (:`A`
        (`self.Crouch`)
        (`/Game/CustomContents/UI/BP/BPC_UserInterface.OnCrounch` _bpc_userinterface true))
      (:`B`
        (`self.UnCrouch`)
        (`/Game/CustomContents/UI/BP/BPC_UserInterface.OnCrounch` _bpc_userinterface false)))))

(event `EnhancedInput|/Game/CustomContents/Input/IA_Sprint`
  (params (ActionValue :type Boolean) (ElapsedSeconds :type "Float (double-precision)") (TriggeredSeconds :type "Float (double-precision)") (InputAction :type "InputAction Object Reference" :default "/Game/CustomContents/Input/IA_Sprint.IA_Sprint"))
  (bind _charactermovement (`self.CharacterMovement`))
  ;[0.04097 0 0.15 0.5] OnInputAction
  ;; OnInputAction_Sprint
  (:`Triggered`
    (set `CharacterMovementComponent.MaxWalkSpeed` 600.0 _charactermovement) ; 달리는 속력
    (set `self.IsSprinting` true))
  (:`Completed`
    (set `CharacterMovementComponent.MaxWalkSpeed` 450.0 _charactermovement) ; 걷는 속력
    (set `self.IsSprinting` false)))

(event `EnhancedInput|/Game/CustomContents/Input/IA_SwitchCam`
  (params (ActionValue :type Boolean) (ElapsedSeconds :type "Float (double-precision)") (TriggeredSeconds :type "Float (double-precision)") (InputAction :type "InputAction Object Reference" :default "/Game/CustomContents/Input/IA_SwitchCam.IA_SwitchCam"))
  ;[0.04097 0 0.15 0.5] OnInputAction
  ;; OnInputAction_SwitchCam
  (:`Triggered`
    (`/Engine/EditorBlueprintResources/StandardMacros.FlipFlop`
      (:`A`
        (`ActorComponent.SetActive` (`self.ThirdPersonCamera`) true false)
        (`ActorComponent.SetActive` (`self.FirstPersonCamera`) false false)
        (set `self.bUseControllerRotationYaw` false))
      (:`B`
        (`ActorComponent.SetActive` (`self.ThirdPersonCamera`) false false)
        (`ActorComponent.SetActive` (`self.FirstPersonCamera`) true false)
        (set `self.bUseControllerRotationYaw` true)))))

(event `EnhancedInput|/Game/CustomContents/Input/IA_Targeting`
  (params (ActionValue :type Boolean) (ElapsedSeconds :type "Float (double-precision)") (TriggeredSeconds :type "Float (double-precision)") (InputAction :type "InputAction Object Reference" :default "/Game/CustomContents/Input/IA_Targeting.IA_Targeting"))
  (bind _bulletspawnlocation (`self.BulletSpawnLocation`))
  (bind _returnvalue (`SceneComponent.K2_GetComponentLocation` _bulletspawnlocation))
  ;[0.04097 0 0.15 0.5] OnInputAction
  ;; OnInputAction_Targeting
  (:`Triggered`
    (bind (_outhit _returnvalue_2) (`KismetSystemLibrary.LineTraceSingleForObjects` :`Start` _returnvalue :`End` (+ _returnvalue (* (`SceneComponent.GetForwardVector` _bulletspawnlocation) 5000.0)) :`ObjectTypes` (`|MakeArray` "ObjectTypeQuery3" :!type "EObjectTypeQuery Enum") :`DrawDebugType` (`self.Debug Enable`)))
    (if _returnvalue_2
      (bind (_bblockinghit _binitialoverlap _time _distance _location _impactpoint _normal _impactnormal _physmat _hitactor _hitcomponent) (`GameplayStatics.BreakHitResult` _outhit))
      (if (`self.ActorHasTag` _hitactor "Enemy")
        (`/Game/CustomContents/UI/BP/BPC_UserInterface.DebugPrintString` (`self.BPC_UserInterface`) "Target Online")
        (set `self.Target` _hitcomponent)))))

(event `EnhancedInput|/Game/CustomContents/Input/IA_HomingFire`
  (params (ActionValue :type Boolean) (ElapsedSeconds :type "Float (double-precision)") (TriggeredSeconds :type "Float (double-precision)") (InputAction :type "InputAction Object Reference" :default "/Game/CustomContents/Input/IA_HomingFire.IA_HomingFire"))
  ;[0.04097 0 0.15 0.5] OnInputAction
  ;; OnInputAction_HomingFrie
  (:`Triggered`
    (`/Engine/EditorBlueprintResources/StandardMacros.IsValid` (`self.Target`)
      (:`Is Valid`
        (for _ (range 8)
          (bind _returnvalue (`|SpawnActorFromClass` "/Game/CustomContents/Blueprints/Weapon/BP_HomingBullet.BP_HomingBullet_C" (`KismetMathLibrary.MakeTransform` (`SceneComponent.K2_GetComponentLocation` (`self.BulletSpawnLocation`))) "Undefined" "MultiplyWithRoot" null null))
          (`/Engine/EditorBlueprintResources/StandardMacros.IsValid` _returnvalue
            (:`Is Valid`
              (set `ProjectileMovementComponent.HomingTargetComponent` (`self.Target`) (`/Game/CustomContents/Blueprints/Weapon/BP_HomingBullet.ProjectileMovement` _returnvalue))
              (`/Game/CustomContents/UI/BP/BPC_UserInterface.DebugPrintString` (`self.BPC_UserInterface`) "Firing"))))))))

(event `EnhancedInput|/Game/CustomContents/Input/IA_Attack_Sandevistan`
  (params (ActionValue :type Boolean) (ElapsedSeconds :type "Float (double-precision)") (TriggeredSeconds :type "Float (double-precision)") (InputAction :type "InputAction Object Reference" :default "/Game/CustomContents/Input/IA_Attack_Sandevistan.IA_Attack_Sandevistan"))
  (bind _bpc_userinterface (`self.BPC_UserInterface`))
  ;[0.04097 0 0.15 0.5] OnInputAction
  ;; Skill_Sandevistan
  (:`Triggered`
    (if (`self.bSandevistan`)
      (set `self.bSandevistan` false)
      (`GameplayStatics.SetGlobalTimeDilation` 1.0)
      (set `self.CustomTimeDilation` 1.0)
      (set `self.SandevistanCnt` 0.0)
      (`/Game/CustomContents/UI/BP/BPC_UserInterface.OnSandevistan` _bpc_userinterface false)
      (elif (>= (`self.SandevistanCnt`) (`self.SandevistanCoolTime`))
        (set `self.bSandevistan` true)
        (`GameplayStatics.SetGlobalTimeDilation` (`self.SandevistanSlowSpeed`))
        (set `self.CustomTimeDilation` (* (`self.SandevistanSlowSpeed`) 10.0))
        (`/Game/CustomContents/UI/BP/BPC_UserInterface.OnSandevistan` _bpc_userinterface true)
        (else
          (`/Game/CustomContents/UI/BP/BPC_UserInterface.DebugPrintString` (`self.BPC_UserInterface`) (`KismetStringLibrary.Concat_StrStr` "쿨타임 : " (`KismetStringLibrary.Conv_DoubleToString` (`self.SandevistanCnt`)))))))))

(fn `DetachWeapon`
  (params (Target :type "Actor Object Reference"))
  (`SceneComponent.K2_DetachFromComponent` (`Actor.RootComponent` Target) "KeepRelative" "KeepRelative" "KeepRelative" true))

(fn `GetDamage`
  (returns (Damage :type "Float (double-precision)") (Critical :type Boolean))
  (bind (_damage _critical) (`/Game/CustomContents/Components/BPC_PlayerStatSystem.GetDamage` (`self.BPC_PlayerStatSystem`)))
  (return _damage _critical))

(fn `SpawnWeaponAndAttach`
  (params (Class :type "Actor Class Reference") (InputPin :type Name))
  (returns (ReturnValue :type "Actor Object Reference"))
  (bind _returnvalue (`|SpawnActorFromClass` Class (`KismetMathLibrary.MakeTransform` (0.0 0.0 0.0)) "Undefined" "MultiplyWithRoot" null null))
  (`self.K2_AttachToComponent` _returnvalue (`self.Mesh`) InputPin "KeepRelative" "KeepRelative" "KeepRelative" true)
  (return _returnvalue))

(fn `UpdatePlayerHealthDisplay`
  (bind _bpc_playerstatsystem (`self.BPC_PlayerStatSystem`))
  ; Update Health Display
  (`/Game/CustomContents/UI/BP/BPC_UserInterface.UpdatePlayerHealth` (`self.BPC_UserInterface`) (`/Game/CustomContents/Components/BPC_PlayerStatSystem.CurrentHealth` _bpc_playerstatsystem) (`/Game/CustomContents/Components/BPC_PlayerStatSystem.MaxHealth` _bpc_playerstatsystem))
  (return))

(fn `UserConstructionScript`)