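; Player character that handles Enhanced Input for look, movement, jump, toggle crouch and hold-to-sprint.
; BeginPlay adds the player mapping context; movement follows control rotation, and sprint switches max walk speed while setting IsSprinting.
; Any damage plays a hit montage and sets IsHitting, which blocks movement input until the montage's then pin clears it.
; Debug prints report damage, crouch and sprint changes.
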(event `self.ReceiveAnyDamage`
  (params (Damage :type "Float (single-precision)") (DamageType :type "DamageType Object Reference") (InstigatedBy :type "Controller Object Reference") (DamageCauser :type "Actor Object Reference"))
  ;[0.15 0 0.02095 0.5] OnDamaged
  (`KismetSystemLibrary.PrintString` "OnDamaged_Player")
  (set `self.IsHitting` true)
  (`|PlayMontage` (`self.Mesh`) "/Game/CustomContents/Animation/Montages/Hit_1_Montage.Hit_1_Montage"
    (:`then`
      (set `self.IsHitting` false))))

(event `self.ReceiveBeginPlay`
  ;[0 0.15 0.008756 0.5] Begin-EnhancedInputAction
  (bind _asplayer_controller (cast `PlayerController` (`self.GetController`)))
  (message `EnhancedInputSubsystemInterface.AddMappingContext` (pcsubsystem `EnhancedInputLocalPlayerSubsystem` _asplayer_controller) "/Game/CustomContents/Input/IMC_Player.IMC_Player" 0 (struct)))

(event `EnhancedInput|/Game/CustomContents/Input/IA_LookAround`
  (params (ActionValue :type "Vector2D Structure") (ElapsedSeconds :type "Float (double-precision)") (TriggeredSeconds :type "Float (double-precision)") (InputAction :type "InputAction Object Reference" :default "/Game/CustomContents/Input/IA_LookAround.IA_LookAround"))
  ;[0.04097 0 0.15 0.5] OnInputAction
  ;; OnInputAction_LookAround
  (:`Triggered`
    (`self.AddControllerYawInput` ActionValue_X)
    (`self.AddControllerPitchInput` ActionValue_Y)))

(event `EnhancedInput|/Game/CustomContents/Input/IA_JumpCustom`
  (params (ActionValue :type Boolean) (ElapsedSeconds :type "Float (double-precision)") (TriggeredSeconds :type "Float (double-precision)") (InputAction :type "InputAction Object Reference" :default "/Game/CustomContents/Input/IA_JumpCustom.IA_JumpCustom"))
  ;[0.04097 0 0.15 0.5] OnInputAction
  ;; OnInputAction_Jump
  (:`Started`
    (`self.Jump`))
  (:`Completed`
    (`self.StopJumping`)))

(event `EnhancedInput|/Game/CustomContents/Input/IA_Movement`
  (params (ActionValue :type "Vector2D Structure") (ElapsedSeconds :type "Float (double-precision)") (TriggeredSeconds :type "Float (double-precision)") (InputAction :type "InputAction Object Reference" :default "/Game/CustomContents/Input/IA_Movement.IA_Movement"))
  (bind (_returnvalue_roll _returnvalue_pitch _returnvalue_yaw) (`KismetMathLibrary.BreakRotator` (`self.GetControlRotation`)))
  (bind (_returnvalue_roll_2 _returnvalue_pitch_2 _returnvalue_yaw_2) (`KismetMathLibrary.BreakRotator` (`self.GetControlRotation`)))
  ;[0.04097 0 0.15 0.5] OnInputAction
  ;; OnInputAction_Movement
  (:`Triggered`
    (if (not (`self.IsHitting`))
      (`self.AddMovementInput` (`KismetMathLibrary.GetRightVector` (`KismetMathLibrary.MakeRotator` _returnvalue_roll_2 0.0 _returnvalue_yaw_2)) ActionValue_X)
      (`self.AddMovementInput` (`KismetMathLibrary.GetForwardVector` (`KismetMathLibrary.MakeRotator` 0.0 0.0 _returnvalue_yaw)) ActionValue_Y))))

(event `EnhancedInput|/Game/CustomContents/Input/IA_Crouch`
  (params (ActionValue :type Boolean) (ElapsedSeconds :type "Float (double-precision)") (TriggeredSeconds :type "Float (double-precision)") (InputAction :type "InputAction Object Reference" :default "/Game/CustomContents/Input/IA_Crouch.IA_Crouch"))
  ;[0.04097 0 0.15 0.5] OnInputAction
  ;; OnInputAction_Crounch
  (:`Started`
    (`/Engine/EditorBlueprintResources/StandardMacros.FlipFlop`
      (:`A`
        (`self.Crouch`)
        (`KismetSystemLibrary.PrintString` "Crounch"))
      (:`B`
        (`self.UnCrouch`)
        (`KismetSystemLibrary.PrintString` "UnCrounch")))))

(event `EnhancedInput|/Game/CustomContents/Input/IA_Sprint`
  (params (ActionValue :type Boolean) (ElapsedSeconds :type "Float (double-precision)") (TriggeredSeconds :type "Float (double-precision)") (InputAction :type "InputAction Object Reference" :default "/Game/CustomContents/Input/IA_Sprint.IA_Sprint"))
  (bind _charactermovement (`self.CharacterMovement`))
  ;[0.04097 0 0.15 0.5] OnInputAction
  ;; OnInputAction_Sprint
  (:`Triggered`
    (set `CharacterMovementComponent.MaxWalkSpeed` 600.0 _charactermovement) ; 달리는 속력
    (set `self.IsSprinting` true)
    (`KismetSystemLibrary.PrintString` "Run"))
  (:`Completed`
    (set `CharacterMovementComponent.MaxWalkSpeed` 450.0 _charactermovement) ; 걷는 속력
    (set `self.IsSprinting` false)
    (`KismetSystemLibrary.PrintString` "Walk")))

(fn `UserConstructionScript`)