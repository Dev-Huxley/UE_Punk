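; Demolitionist gunner fire-shot projectile that damages enemies and plays a Niagara impact effect on contact.
; Sphere overlap with a BP_Enemy applies damage and critical values from the player's stat system, with the cached player controller as instigator.
; Collision hits call CallOnComponenetHit and spawn the impact at the hit point; either contact destroys the projectile.
; Otherwise it self-destroys after a short lifetime; the blood effect is unwired.
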(event `self.ReceiveBeginPlay`
  ; SetPlayerCharacter
  (bind _asbp_player_character (cast `/Game/CustomContents/Blueprints/Character/Player/BP_PlayerCharacter` (`Controller.K2_GetPawn` (`GameplayStatics.GetPlayerController` 0))))
  (set `self.BP_PlayerCharacter` _asbp_player_character)
  ; 총알 생성 후 2.5초 destroy
  (`KismetSystemLibrary.Delay` 2.5)
  (`GameplayStatics.SpawnEmitterAtLocation` null)
  (`self.K2_DestroyActor`))

(event `self.Sphere.OnComponentBeginOverlap`
  (params (OverlappedComponent :type "PrimitiveComponent Object Reference") (OtherActor :type "Actor Object Reference") (OtherComp :type "PrimitiveComponent Object Reference") (OtherBodyIndex :type Integer) (bFromSweep :type Boolean) (SweepResult :type "HitResult Structure (by ref)"))
  ; Enemy태그 체크하고 맞다면 destroy+emitter
  (bind _asbp_enemy (cast `/Game/CustomContents/Blueprints/Character/Enemy/BP_Enemy` OtherActor))
  (bind (_damage _critical) (`/Game/CustomContents/Components/BPC_PlayerStatSystem.GetBulletDamage` (`/Game/CustomContents/Blueprints/Character/Player/BP_PlayerCharacter.BPC_PlayerStatSystem` (`self.BP_PlayerCharacter`))))
  (`/Game/CustomContents/Blueprints/Character/Enemy/BP_Enemy.OnDamage` _asbp_enemy _damage _critical (`Pawn.GetController` (`self.BP_PlayerCharacter`)) self)
  (`NiagaraFunctionLibrary.SpawnSystemAtLocation` "/Game/POLYMORPHFX/DemolitionistGunnerFireShotVFX/Niagara/NS_Demolitionist_Gunner_FireShot_Impact_01.NS_Demolitionist_Gunner_FireShot_Impact_01")
  (`self.K2_DestroyActor`))

(event `self.Collision.OnComponentHit`
  (params (HitComponent :type "PrimitiveComponent Object Reference") (OtherActor :type "Actor Object Reference") (OtherComp :type "PrimitiveComponent Object Reference") (NormalImpulse :type "Vector Structure") (Hit :type "HitResult Structure (by ref)"))
  (`self.OnComponenetHit` OtherActor Hit)
  (`NiagaraFunctionLibrary.SpawnSystemAtLocation` "/Game/POLYMORPHFX/DemolitionistGunnerFireShotVFX/Niagara/NS_Demolitionist_Gunner_FireShot_Impact_01.NS_Demolitionist_Gunner_FireShot_Impact_01" (`.Location` (`GameplayStatics.BreakHitResult` Hit)))
  (`self.K2_DestroyActor`))

(fn `UserConstructionScript`)